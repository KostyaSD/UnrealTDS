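; Top-down player character with a configurable boom camera and an aim control.
; Holding the right mouse button switches the movement state to aim, and releasing it switches to run.
; The construction script applies camera height, rotation and lag smoothing variables to the camera boom.
; A separate shake function plays a world camera shake centred on the top-down camera's location.
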(event `Key|RightMouseButton`
  (params (Key :type "Key Structure"))
  (:`Pressed`
    (`self.ChangeMovementState` "Aim_State"))
  (:`Released`
    (`self.ChangeMovementState` "Run_State")))

(fn `CameraShakeEvent`
  (`GameplayStatics.PlayWorldCameraShake` "/Game/Blueprints/Game/BP_ShakeCamera.BP_ShakeCamera_C" (`SceneComponent.K2_GetComponentLocation` (`self.TopDownCameraComponent`)) 0.0 30.0))

(fn `UserConstructionScript`
  (bind _cameraboom (`self.CameraBoom`))
  (set `SpringArmComponent.TargetArmLength` (`self.Hieght`) _cameraboom)
  (`SceneComponent.K2_SetRelativeRotation` _cameraboom (`self.RotatorCamera`) false false)
  (set `SpringArmComponent.bEnableCameraLag` (`self.Flow`) _cameraboom)
  (set `SpringArmComponent.CameraLagSpeed` (`self.CoefSmoot`) _cameraboom))